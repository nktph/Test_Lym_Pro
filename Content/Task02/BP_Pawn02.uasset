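; BP_Pawn02 is a Task02 pawn that relays numpad input to the BP_RopeSphere found in the level.
; Holding NumPad 4 or 6 repeatedly calls RopeUp or RopeDown through a self-re-entering Gate and short RetriggerableDelay loop, until key release closes the Gate.
; NumPad 2 and 3 call Speed2 and Speed1 respectively and print the selected speed.
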(event EventBeginPlay)

(event Collision|EventActorBeginOverlap
  (params (OtherActor :type Actor%20Object%20Reference)))

(event EventTick
  (params (DeltaSeconds :type Float%20%28single-precision%29)))

(event Input|KeyboardEvents|NumPadFour
  (params (Key :type Key%20Structure :default "None"))
  ;[1 1 1] ROPE +/-
  (:Pressed
    (Utilities|FlowControl|Sequence
      (:then_0
        (goto _label Open))
      (:then_1
        (Utilities|FlowControl|Gate true :!label _label
          (:Exit
            (bind _returnvalue (Actor|GetActorOfClass "/Game/Task02/BP_RopeSphere.BP_RopeSphere_C"))
            (Utilities|IsValid _returnvalue
              (:Is%20Valid
                (Default|RopeUp _returnvalue)
                (Utilities|FlowControl|RetriggerableDelay 0.1)
                (goto _label))))))))
  (:Released
    (goto _label Close)))

(event Input|KeyboardEvents|NumPadSix
  (params (Key :type Key%20Structure :default "None"))
  ;[1 1 1] ROPE +/-
  (:Pressed
    (Utilities|FlowControl|Sequence
      (:then_0
        (goto _label Open))
      (:then_1
        (Utilities|FlowControl|Gate true :!label _label
          (:Exit
            (bind _returnvalue (Actor|GetActorOfClass "/Game/Task02/BP_RopeSphere.BP_RopeSphere_C"))
            (Utilities|IsValid _returnvalue
              (:Is%20Valid
                (Default|RopeDown _returnvalue)
                (Utilities|FlowControl|RetriggerableDelay 0.1)
                (goto _label))))))))
  (:Released
    (goto _label Close)))

(event Input|KeyboardEvents|NumPadTwo
  (params (Key :type Key%20Structure :default "None"))
  ;[1 1 1] Speed
  (:Pressed
    (bind _returnvalue (Actor|GetActorOfClass "/Game/Task02/BP_RopeSphere.BP_RopeSphere_C"))
    (Utilities|IsValid _returnvalue
      (:Is%20Valid
        (Default|Speed2 _returnvalue)
        (Development|PrintString "Speed = 2")))))

(event Input|KeyboardEvents|NumPadThree
  (params (Key :type Key%20Structure :default "None"))
  ;[1 1 1] Speed
  (:Pressed
    (bind _returnvalue (Actor|GetActorOfClass "/Game/Task02/BP_RopeSphere.BP_RopeSphere_C"))
    (Utilities|IsValid _returnvalue
      (:Is%20Valid
        (Default|Speed1 _returnvalue)
        (Development|PrintString "Speed = 1")))))

(fn ConstructionScript)
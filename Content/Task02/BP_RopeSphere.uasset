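; BP_RopeSphere is a sphere on an adjustable rope, built from a cable and a physics constraint.
; RopeUp and RopeDown events shorten or lengthen the cable by a speed-scaled step within a clamped range, matching the constraint's linear Z limit to the new length.
; Speed1 and Speed2 events switch that step's multiplier.
; BeginPlay nudges the sphere sideways from its starting position.
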(event Custom|RopeUp
  (CallFunction|RopeShorter))

(event Custom|RopeDown
  (CallFunction|RopeLonger))

(event Custom|Speed2
  (CallFunction|RopeSpeed 2.0))

(event Custom|Speed1
  (CallFunction|RopeSpeed 1.0))

(event EventBeginPlay
  (Transformation|AddWorldOffset (Variables|Default|GetSphere) "0.000000,-300.000000,0.000000" false false))

(event Collision|EventActorBeginOverlap
  (params (OtherActor :type Actor%20Object%20Reference)))

(event EventTick
  (params (DeltaSeconds :type Float%20%28single-precision%29)))

(fn ConstructionScript)

(fn RopeSpeed
  (params (Speed :type Float%20%28double-precision%29))
  (Variables|Default|SetSpeed Speed))

(fn RopeShorter
  (bind _cable (Variables|Default|GetCable))
  (bind _output_get (Variables|/Script/CableComponent.CableComponent|SetCableLength _cable (Math|Float|Clamp(Float) (- (Variables|/Script/CableComponent.CableComponent|GetCableLength _cable) (* (Variables|Default|GetSpeed) 5.0)) 0.0 4e+02)))
  (Class|PhysicsConstraintComponent|SetLinearZLimit (Variables|Default|GetRopeConstraint) "LCM_Limited" _output_get))

(fn RopeLonger
  (bind _cable (Variables|Default|GetCable))
  (bind _output_get (Variables|/Script/CableComponent.CableComponent|SetCableLength _cable (Math|Float|Clamp(Float) (+ (Variables|/Script/CableComponent.CableComponent|GetCableLength _cable) (* (Variables|Default|GetSpeed) 5.0)) 0.0 4e+02)))
  (Class|PhysicsConstraintComponent|SetLinearZLimit (Variables|Default|GetRopeConstraint) "LCM_Limited" _output_get))
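; BP_Sphere is a sphere that animates fading in and out and switching an emissive glow on and off.
; BeginPlay creates a dynamic M_Sphere material instance, starting opaque and unlit by emission.
; FadeIn and FadeOut timelines, paced by ShowAnimPlayRate, drive opacity and shift the root vertically from the sphere's captured location.
; One Emission timeline plays forward for EmmitOn and reverses from its end for EmmitOff, clamped to MaxEmissive.
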(event Custom|FadeIn
  ;[1 1 1] Fade In
  (bind _output_get (Variables|Default|SetLocation (Transformation|GetWorldLocation (Variables|Default|GetSphere))))
  (Components|Timeline|SetPlayRate (Variables|Default|GetFade_In) (Variables|Default|GetShowAnimPlayRate))
  (bind (_direction _opacity _zoffset) (Timeline|Fade_In PlayFromStart)
    (:Update
      (Rendering|Material|SetScalarParameterValue (Variables|Default|GetSphereMaterial) "Opacity" _opacity :!class /Script/Engine.MaterialInstanceDynamic)
      (Transformation|SetWorldLocation (Variables|Default|GetDefaultSceneRoot) (Math|Vector|MakeVector (.X (Class|KismetMathLibrary|BreakVector3f _output_get)) (.Y (Class|KismetMathLibrary|BreakVector3f _output_get)) (+ (.Z (Class|KismetMathLibrary|BreakVector3f _output_get)) _zoffset)) false false))))

(event Custom|FadeOut
  ;[1 1 1] Fade Out
  (bind _output_get (Variables|Default|SetLocation (Transformation|GetWorldLocation (Variables|Default|GetSphere))))
  (Components|Timeline|SetPlayRate (Variables|Default|GetFade_Out) (Variables|Default|GetShowAnimPlayRate))
  (bind (_direction _opacity _zposition) (Timeline|Fade_Out PlayFromStart)
    (:Update
      (Rendering|Material|SetScalarParameterValue (Variables|Default|GetSphereMaterial) "Opacity" _opacity :!class /Script/Engine.MaterialInstanceDynamic)
      (Transformation|SetWorldLocation (Variables|Default|GetDefaultSceneRoot) (Math|Vector|MakeVector (.X (Class|KismetMathLibrary|BreakVector3f _output_get)) (.Y (Class|KismetMathLibrary|BreakVector3f _output_get)) (+ (.Z (Class|KismetMathLibrary|BreakVector3f _output_get)) _zposition)) false false))))

(event Custom|EmmitOn
  ;[1 1 1] Emission ON/OFF
  (bind _emission (Timeline|Emission PlayFromStart)
    (:Update
      (Rendering|Material|SetScalarParameterValue (Variables|Default|GetSphereMaterial) "Emission" (Math|Float|Clamp(Float) _emission 0.0 (Variables|Default|GetMaxEmissive)) :!class /Script/Engine.MaterialInstanceDynamic))))

(event Custom|EmmitOff
  ;[1 1 1] Emission ON/OFF
  (bind _emission (Timeline|Emission ReverseFromEnd)
    (:Update
      (Rendering|Material|SetScalarParameterValue (Variables|Default|GetSphereMaterial) "Emission" (Math|Float|Clamp(Float) _emission 0.0 (Variables|Default|GetMaxEmissive)) :!class /Script/Engine.MaterialInstanceDynamic))))

(event EventBeginPlay
  (bind _returnvalue (Rendering|Material|CreateDynamicMaterialInstance (Variables|Default|GetSphere) 0 "/Game/Task01/M_Sphere.M_Sphere" "None" :!class /Script/Engine.PrimitiveComponent))
  (bind _output_get (Variables|Default|SetSphereMaterial _returnvalue))
  (Rendering|Material|SetScalarParameterValue _output_get "Opacity" 1.0 :!class /Script/Engine.MaterialInstanceDynamic)
  (Rendering|Material|SetScalarParameterValue _output_get "Emission" 0.0 :!class /Script/Engine.MaterialInstanceDynamic))

(fn ConstructionScript)
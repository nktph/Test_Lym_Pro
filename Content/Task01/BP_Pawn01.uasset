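; BP_Pawn01 is a pawn that serves as a keyboard test controller for BP_Sphere's visual effects.
; NumPad 0 and 1 call FadeIn and FadeOut on the sphere, while NumPad 2 and 3 call EmmitOn and EmmitOff.
; Each key press looks up the sphere with GetActorOfClass and checks validity before calling it.
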(event EventBeginPlay)

(event Collision|EventActorBeginOverlap
  (params (OtherActor :type Actor%20Object%20Reference)))

(event EventTick
  (params (DeltaSeconds :type Float%20%28single-precision%29)))

(event Input|KeyboardEvents|NumPadTwo
  (params (Key :type Key%20Structure :default "None"))
  ;[1 1 1] EmmitOn-EmmitOff
  (:Pressed
    (bind _returnvalue (Actor|GetActorOfClass "/Game/Task01/BP_Sphere.BP_Sphere_C"))
    (Utilities|IsValid _returnvalue
      (:Is%20Valid
        (Default|Emmiton _returnvalue)))))

(event Input|KeyboardEvents|NumPadThree
  (params (Key :type Key%20Structure :default "None"))
  ;[1 1 1] EmmitOn-EmmitOff
  (:Pressed
    (bind _returnvalue (Actor|GetActorOfClass "/Game/Task01/BP_Sphere.BP_Sphere_C"))
    (Utilities|IsValid _returnvalue
      (:Is%20Valid
        (Default|EmmitOff _returnvalue)))))

(event Input|KeyboardEvents|NumPadZero
  (params (Key :type Key%20Structure :default "None"))
  ;[1 1 1] Appear-Fade
  (:Pressed
    (bind _returnvalue (Actor|GetActorOfClass "/Game/Task01/BP_Sphere.BP_Sphere_C"))
    (Utilities|IsValid _returnvalue
      (:Is%20Valid
        (Default|Fadein _returnvalue)))))

(event Input|KeyboardEvents|NumPadOne
  (params (Key :type Key%20Structure :default "None"))
  ;[1 1 1] Appear-Fade
  (:Pressed
    (bind _returnvalue (Actor|GetActorOfClass "/Game/Task01/BP_Sphere.BP_Sphere_C"))
    (Utilities|IsValid _returnvalue
      (:Is%20Valid
        (Default|FadeOut _returnvalue)))))

(fn ConstructionScript)